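; Dungeon doorway whose right door leaf is swung by a grabbing hand component, likely VR.
; Grab stores the component if it lies within SphereRight's radius, and Release clears it.
; Tick sets Locked when the door's world yaw is essentially zero.
; Only while Locked, the door yaws toward the hand via look-at, clamped to a half-turn, or snaps closed without one, so movement stops once yaw leaves zero.
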(event EventBeginPlay)

(event Collision|EventActorBeginOverlap
  (params (OtherActor :type Actor%20Object%20Reference)))

(event EventRelease
  (params (Component :type Motion%20Controller%20Component%20Object%20Reference))
  (if (== Component (Variables|Default|GetHand))
    (Variables|Default|SetHand 0)))

(event EventGrab
  (params (Component :type Motion%20Controller%20Component%20Object%20Reference))
  (bind _sphereright (Variables|Default|GetSphereRight))
  (if (Utilities|Operators|EqualEqual (Transformation|GetWorldLocation Component) (Transformation|GetWorldLocation _sphereright) (Variables|/Script/Engine.SphereComponent|GetSphereRadius _sphereright))
    (Variables|Default|SetHand Component)))

(event EventTick
  (params (DeltaSeconds :type Float%20%28single-precision%29))
  (bind _hand (Variables|Default|GetHand))
  (bind _sm_doorway_large_door_right (Variables|Default|GetSM_DoorWay_Large_Door_Right))
  (Utilities|FlowControl|Sequence
    (:then_0
      (if (Math|Float|NearlyEqual(Float) (.yaw (Transformation|GetWorldRotation (Variables|Default|GetSM_DoorWay_Large_Door_Right))) 0.0 1e-06)
        (Variables|Default|Setlocked true)
        (else
          (Variables|Default|Setlocked false))))
    (:then_1
      (if (Variables|Default|Getlocked)
        (Utilities|IsValid _hand
          (:Is%20Valid
            (Transformation|SetWorldRotation _sm_doorway_large_door_right (Math|Rotator|MakeRotator 0.0 0.0 (Math|Float|ClampAngle (- (.yaw (Math|Rotator|FindLookatRotation (Transformation|GetWorldLocation _hand) (Transformation|GetWorldLocation _sm_doorway_large_door_right))) 9e+01) -9e+01 9e+01)) false false))
          (:Is%20Not%20Valid
            (if (Math|Float|NearlyEqual(Float) (.yaw (Transformation|GetWorldRotation _sm_doorway_large_door_right)) 0.0 1e+01)
              (Transformation|SetWorldRotation _sm_doorway_large_door_right "0, 0, 0" false false))))))))

(fn ConstructionScript)