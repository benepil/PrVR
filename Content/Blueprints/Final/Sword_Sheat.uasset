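; VR sword sheath that guides a sword along a spline-defined straight path and triggers the win when it reaches the far end.
; Each tick it checks for a sword overlapping one endpoint, then detaches itself and constrains that sword to the segment at the closest point to its motion controller.
; At the other endpoint it snaps the sword back to the controller, then after short delays plays a win sound and opens the winner screen.
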(event EventBeginPlay
  (bind _spline (Variables|Default|GetSpline))
  (Variables|Default|SetStartPoint (Spline|GetLocationatSplinePoint _spline 1 "World"))
  (Variables|Default|SetEndPoint (Spline|GetLocationatSplinePoint _spline 0 "World")))

(event EventTick
  (params (DeltaSeconds :type Float%20%28single-precision%29))
  (bind _startpoint (Variables|Default|GetStartPoint))
  (Utilities|IsValid (Variables|Default|GetSword)
    (:Is%20Valid
      (Utilities|IsValid (Variables|/Game/Blueprints/Final/Sword.Sword_C|GetMotion%20Controller (Variables|Default|GetSword))
        (:Is%20Valid
          (Transformation|SetActorLocation (Variables|Default|GetSword) (Math|Vector|FindClosestPointonSegment (Transformation|GetWorldLocation (Variables|/Game/Blueprints/Final/Sword.Sword_C|GetMotion%20Controller (Variables|Default|GetSword))) _startpoint (Variables|Default|GetEndPoint)) false false)
          (if (Utilities|Operators|EqualEqual (Transformation|GetActorLocation (Variables|Default|GetSword)) _startpoint 1e+01)
            (Transformation|AttachComponentToComponent (Variables|Default|GetSword) (Variables|/Game/Blueprints/Final/Sword.Sword_C|GetMotion%20Controller (Variables|Default|GetSword)) "None" "SnapToTarget" "SnapToTarget" "KeepWorld" true)
            (Variables|Default|SetSword 0)
            (Utilities|FlowControl|Delay 2.0)
            (Audio|PlaySound2D "/Game/Audio/WinSound_Cue.WinSound_Cue" 1.0 1.0 0.0 0 0)
            (Utilities|FlowControl|Delay 0.2)
            (Game|OpenLevel(byObjectReference) "/Game/Maps/WinnerScreen.WinnerScreen")))
        (:Is%20Not%20Valid)))
    (:Is%20Not%20Valid
      (bind _outactors (Collision|SphereOverlapActors (Variables|Default|GetEndPoint) 2e+01 (Utilities|Array|MakeArray "ObjectTypeQuery2") 0))
      (bind _array_element (Utilities|Array|ForEachLoopwithBreak _outactors :!label _label)
        (:LoopBody
          (bind _assword (Utilities|Casting|CastToSword _array_element))
          (Variables|Default|SetSword _assword)
          (Transformation|DetachFromActor "KeepWorld" "KeepWorld" "KeepWorld")
          (goto _label Break))))))

(fn ConstructionScript)