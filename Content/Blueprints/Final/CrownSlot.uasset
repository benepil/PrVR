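; CrownSlot is a snap slot that previews where a Crown can be placed, using a ghost mesh.
; When a Crown enters the sphere and no SnapObject is set, it is stored and CrownMesh copies its mesh and scale with the GhostMesh material.
; When that Crown leaves, the mesh and reference are cleared.
; AttachToSlot hides the preview and DetachFromSlot shows it again; construction starts it hidden.
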(event OnComponentBeginOverlap(Sphere)
  (params (OverlappedComponent :type Primitive%20Component%20Object%20Reference) (OtherActor :type Actor%20Object%20Reference) (OtherComp :type Primitive%20Component%20Object%20Reference) (OtherBodyIndex :type Integer) (bFromSweep :type Boolean) (SweepResult :type Hit%20Result%20Structure%20%28by%20ref%29))
  (bind _ascrown (Utilities|Casting|CastToCrown OtherActor))
  (Utilities|IsValid (Variables|Default|GetSnapObject)
    (:Is%20Not%20Valid
      (bind _output_get (Variables|Default|SetSnapObject _ascrown))
      (Components|StaticMesh|SetStaticMesh (Variables|Default|GetCrownMesh) (Variables|/Script/Engine.StaticMeshComponent|GetStaticMesh (Variables|/Game/Blueprints/Final/Crown.Crown_C|GetStaticMesh _output_get)))
      (Transformation|SetWorldScale3D (Variables|Default|GetCrownMesh) (Transformation|GetWorldScale (Variables|/Game/Blueprints/Final/Crown.Crown_C|GetStaticMesh _output_get)))
      (Rendering|SetVisibility (Variables|Default|GetCrownMesh) true false)
      (for _index (range 0 (- (Rendering|Material|GetNumMaterials (Variables|Default|GetCrownMesh)) 1))
        (Rendering|Material|SetMaterial (Variables|Default|GetCrownMesh) _index (Variables|Default|GetGhostMesh))))))

(event OnComponentEndOverlap(Sphere)
  (params (OverlappedComponent :type Primitive%20Component%20Object%20Reference) (OtherActor :type Actor%20Object%20Reference) (OtherComp :type Primitive%20Component%20Object%20Reference) (OtherBodyIndex :type Integer))
  (bind _ascrown (Utilities|Casting|CastToCrown OtherActor))
  (if (== _ascrown (Variables|Default|GetSnapObject))
    (Components|StaticMesh|SetStaticMesh (Variables|Default|GetCrownMesh) 0)
    (Variables|Default|SetSnapObject 0)))

(event Custom|AttachToSlot
  (Rendering|SetVisibility (Variables|Default|GetCrownMesh) false false))

(event Custom|DetachFromSlot
  (Rendering|SetVisibility (Variables|Default|GetCrownMesh) true false))

(fn ConstructionScript
  (Rendering|SetVisibility (Variables|Default|GetCrownMesh) false false))