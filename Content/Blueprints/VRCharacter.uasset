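; VR player character that handles left-thumbstick movement and grabbing objects with both motion controllers.
; Movement follows the left controller's forward and right vectors, while grab and release go through GrippableInterface messages.
; The left hand messages every grippable in its sphere component, storing the last for release.
; The right hand grabs the first from a WorldDynamic sphere overlap query, leaving its component-based version disconnected.
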(event Input|ActionEvents|InputActionGrabLeft
  (params (Key :type Key%20Structure :default "None"))
  (:Pressed
    (for _array_element (Collision|GetOverlappingActors (Variables|Components|GetSphereLeft) 0 :!class /Script/Engine.PrimitiveComponent)
      (if (Utilities|DoesObjectImplementInterface _array_element "/Game/Interface/GrippableInterface.GrippableInterface_C")
        (Class|GrippableInterface|Grab(Message) _array_element (Variables|Components|GetMotionControllerLeft))
        (Variables|Default|SetGrabLeftActor _array_element))))
  (:Released
    (Utilities|IsValid (Variables|Default|GetGrabLeftActor)
      (:Is%20Valid
        (Class|GrippableInterface|Release(Message) (Variables|Default|GetGrabLeftActor))))))

(event Input|ActionEvents|InputActionGrabRight
  (params (Key :type Key%20Structure :default "None")))

(event Input|ActionEvents|InputActionGrabRight
  (params (Key :type Key%20Structure :default "None"))
  (:Pressed
    (bind _outactors (Collision|SphereOverlapActors (Transformation|GetWorldLocation (Variables|Components|GetMotionControllerRight)) 2e+01 (Utilities|Array|MakeArray "ObjectTypeQuery2") 0))
    (bind _array_element (Utilities|Array|ForEachLoopwithBreak _outactors :!label _label)
      (:LoopBody
        (if (Utilities|DoesObjectImplementInterface _array_element "/Game/Interface/GrippableInterface.GrippableInterface_C")
          (bind _output_get (Variables|Default|SetGrabRight _array_element))
          (Class|GrippableInterface|Grab(Message) _output_get (Variables|Components|GetMotionControllerRight))
          (goto _label Break)))))
  (:Released
    (Class|GrippableInterface|Release(Message) (Variables|Default|GetGrabRight) (Variables|Components|GetMotionControllerRight))))

(event Input|AxisEvents|InputAxisMotionControllerThumbLeft_X
  (params (AxisValue :type Float%20%28single-precision%29))
  (Pawn|Input|AddMovementInput (Math|Vector|GetRightVector (Variables|Components|GetMotionControllerLeft)) AxisValue false))

(event Input|AxisEvents|InputAxisMotionControllerThumbLeft_Y
  (params (AxisValue :type Float%20%28single-precision%29))
  (Pawn|Input|AddMovementInput (Math|Vector|GetForwardVector (Variables|Components|GetMotionControllerLeft)) AxisValue false))

(fn ConstructionScript)