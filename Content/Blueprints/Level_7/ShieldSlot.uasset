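; ShieldSlot is a snap slot that previews where a Shield can be placed.
; When a Shield enters its sphere and no snap object is held, it stores that Shield and shows a copy of its mesh and scale with a ghost material on every slot.
; Attach and detach events hide and show the ghost, and the stored Shield leaving the sphere clears it.
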(event OnComponentBeginOverlap(Sphere)
  (params (OverlappedComponent :type Primitive%20Component%20Object%20Reference) (OtherActor :type Actor%20Object%20Reference) (OtherComp :type Primitive%20Component%20Object%20Reference) (OtherBodyIndex :type Integer) (bFromSweep :type Boolean) (SweepResult :type Hit%20Result%20Structure%20%28by%20ref%29))
  (bind _asshield (Utilities|Casting|CastToShield OtherActor))
  (Utilities|IsValid (Variables|Default|GetSnapObject)
    (:Is%20Not%20Valid
      (bind _output_get (Variables|Default|SetSnapObject _asshield))
      (Components|StaticMesh|SetStaticMesh (Variables|Default|GetShieldMesh) (Variables|/Script/Engine.StaticMeshComponent|GetStaticMesh (Variables|/Game/Blueprints/Level_7/Shield.Shield_C|GetStaticMesh _output_get)))
      (Transformation|SetWorldScale3D (Variables|Default|GetShieldMesh) (Transformation|GetWorldScale (Variables|/Game/Blueprints/Level_7/Shield.Shield_C|GetStaticMesh _output_get)))
      (Rendering|SetVisibility (Variables|Default|GetShieldMesh) true false)
      (for _index (range 0 (- (Rendering|Material|GetNumMaterials (Variables|Default|GetShieldMesh)) 1))
        (Rendering|Material|SetMaterial (Variables|Default|GetShieldMesh) _index (Variables|Default|GetGhostMesh))))))

(event OnComponentEndOverlap(Sphere)
  (params (OverlappedComponent :type Primitive%20Component%20Object%20Reference) (OtherActor :type Actor%20Object%20Reference) (OtherComp :type Primitive%20Component%20Object%20Reference) (OtherBodyIndex :type Integer))
  (bind _asshield (Utilities|Casting|CastToShield OtherActor))
  (if (== _asshield (Variables|Default|GetSnapObject))
    (Components|StaticMesh|SetStaticMesh (Variables|Default|GetShieldMesh) 0)
    (Variables|Default|SetSnapObject 0)))

(event Custom|AttachToSlot
  (Rendering|SetVisibility (Variables|Default|GetShieldMesh) false false))

(event Custom|DetachFromSlot
  (Rendering|SetVisibility (Variables|Default|GetShieldMesh) true false))

(fn ConstructionScript
  (Rendering|SetVisibility (Variables|Default|GetShieldMesh) false false))