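; A VR-grabbable shield actor for Level 7 that can be placed into a ShieldSlot.
; Grabbing attaches it to the motion controller and turns off mesh physics; releasing detaches it.
; Mesh overlaps with a slot's sphere track the candidate slot.
; Releasing over a slot notifies it, snaps the shield to the slot's shield mesh transform and flags it as in place.
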(event OnComponentBeginOverlap(StaticMesh)
  (params (OverlappedComponent :type Primitive%20Component%20Object%20Reference) (OtherActor :type Actor%20Object%20Reference) (OtherComp :type Primitive%20Component%20Object%20Reference) (OtherBodyIndex :type Integer) (bFromSweep :type Boolean) (SweepResult :type Hit%20Result%20Structure%20%28by%20ref%29))
  (bind _asshield_slot (Utilities|Casting|CastToShieldSlot OtherActor))
  (if (== (Variables|/Game/Blueprints/Level_7/ShieldSlot.ShieldSlot_C|GetSphere _asshield_slot) OtherComp)
    (Variables|Default|SetSlot _asshield_slot)))

(event OnComponentEndOverlap(StaticMesh)
  (params (OverlappedComponent :type Primitive%20Component%20Object%20Reference) (OtherActor :type Actor%20Object%20Reference) (OtherComp :type Primitive%20Component%20Object%20Reference) (OtherBodyIndex :type Integer))
  (Utilities|IsValid (Variables|Default|GetSlot)
    (:Is%20Valid
      (bind _asshield_slot (Utilities|Casting|CastToShieldSlot OtherActor))
      (if (and (== (Variables|/Game/Blueprints/Level_7/ShieldSlot.ShieldSlot_C|GetSphere _asshield_slot) OtherComp) (== _asshield_slot (Variables|Default|GetSlot)))
        (Variables|Default|SetSlot 0)))))

(event EventGrab
  (params (Component :type Motion%20Controller%20Component%20Object%20Reference))
  (bind _output_get (Variables|Default|SetMotion%20Controller Component))
  (Transformation|AttachComponentToComponent _output_get "None" "KeepWorld" "KeepWorld" "KeepWorld" true)
  (Physics|SetSimulatePhysics (Variables|Default|GetStaticMesh) false))

(event EventRelease
  (params (Component :type Motion%20Controller%20Component%20Object%20Reference))
  (bind _slot (Variables|Default|GetSlot))
  (bind _shieldmesh (Variables|/Game/Blueprints/Level_7/ShieldSlot.ShieldSlot_C|GetShieldMesh _slot))
  (Variables|Default|SetMotion%20Controller 0)
  (Transformation|DetachFromActor "KeepWorld" "KeepWorld" "KeepWorld")
  (Utilities|IsValid _slot
    (:Is%20Valid
      (Default|AttachtoSlot _slot)
      (Transformation|SetActorLocationAndRotation (Transformation|GetWorldLocation _shieldmesh) (Transformation|GetWorldRotation _shieldmesh))
      (Variables|Default|SetInPlace true))))

(fn ConstructionScript)