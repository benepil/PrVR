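; VR padlock that unlocks when a key is slid into it along a two-point spline.
; Tick captures a Key overlapping the outer point, detaches it, and constrains it to the segment by projecting the motion controller's position.
; Pulling back to the outer point returns the key to the controller.
; Releasing it at the inner end unlocks, attaching the key, enabling physics and playing a sound, while releasing elsewhere drops it.
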(event EventBeginPlay
  (bind _spline (Variables|Default|GetSpline))
  (Variables|Default|SetStartPoint (Spline|GetLocationatSplinePoint _spline 1 "World"))
  (Variables|Default|SetEndPoint (Spline|GetLocationatSplinePoint _spline 0 "World"))
  (Variables|Default|SetLocked true))

(event EventTick
  (params (DeltaSeconds :type Float%20%28single-precision%29))
  (bind _startpoint (Variables|Default|GetStartPoint))
  (Utilities|IsValid (Variables|Default|GetKey)
    (:Is%20Valid
      (Utilities|IsValid (Variables|/Game/Blueprints/Level_3/Key.Key_C|GetMotion%20Controller (Variables|Default|GetKey))
        (:Is%20Valid
          (Transformation|SetActorLocationAndRotation (Variables|Default|GetKey) (Math|Vector|FindClosestPointonSegment (Transformation|GetWorldLocation (Variables|/Game/Blueprints/Level_3/Key.Key_C|GetMotion%20Controller (Variables|Default|GetKey))) _startpoint (Variables|Default|GetEndPoint)) "90.000000,90.000000,0.000000")
          (if (Utilities|Operators|EqualEqual (Transformation|GetActorLocation (Variables|Default|GetKey)) _startpoint 1e+01)
            (Transformation|AttachComponentToComponent (Variables|Default|GetKey) (Variables|/Game/Blueprints/Level_3/Key.Key_C|GetMotion%20Controller (Variables|Default|GetKey)) "None" "SnapToTarget" "KeepWorld" "KeepWorld" true)
            (Variables|Default|SetKey 0)
            (Variables|Default|SetLocked true)))
        (:Is%20Not%20Valid
          (if (Utilities|Operators|EqualEqual (Transformation|GetActorLocation (Variables|Default|GetKey)) (Variables|Default|GetEndPoint) 5.0)
            (Variables|Default|SetLocked false)
            (Transformation|SetActorLocationAndRotation (Variables|Default|GetKey) (Variables|Default|GetEndPoint) "90.000000,90.000000,0.000000")
            (Transformation|AttachActorToActor (Variables|Default|GetKey) self "None" "KeepWorld" "KeepWorld" "KeepWorld" true)
            (Physics|SetSimulatePhysics (Variables|Default|GetLock) true)
            (Audio|PlaySound2D "/Game/Audio/Unlock_padlock_Cue.Unlock_padlock_Cue" 1.0 1.0 0.0 0 0)
            (else
              (Physics|SetSimulatePhysics (Variables|/Game/Blueprints/Level_3/Key.Key_C|GetKey%20Mesh (Variables|Default|GetKey)) true)
              (Variables|Default|SetKey 0))))))
    (:Is%20Not%20Valid
      (bind _outactors (Collision|SphereOverlapActors (Variables|Default|GetStartPoint) 2e+01 (Utilities|Array|MakeArray "ObjectTypeQuery2") 0))
      (bind _array_element (Utilities|Array|ForEachLoopwithBreak _outactors :!label _label)
        (:LoopBody
          (bind _askey (Utilities|Casting|CastToKey _array_element))
          (bind _output_get (Variables|Default|SetKey _askey))
          (Transformation|DetachFromActor _output_get "KeepWorld" "KeepWorld" "KeepWorld")
          (goto _label Break))))))

(fn ConstructionScript)