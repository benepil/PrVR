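; BP_FireCoals is a Level 6 fire coals actor that burns objects and cycles its light color, apparently as part of an unlock puzzle.
; Every tick, a sphere overlap finds world-dynamic actors implementing BurnInterface and sends them BurnMessage.
; After a burn, the point light steps through red, yellow and green, using its current color as the state.
; Unlocked turns true only on the step back to red.
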(event EventTick
  (params (DeltaSeconds :type Float%20%28single-precision%29))
  (bind _sphere (Variables|Default|GetSphere))
  (bind _pointlight (Variables|Default|GetPointLight))
  (bind _returnvalue (Rendering|Components|Light|GetLightColor _pointlight))
  (bind _outactors (Collision|SphereOverlapActors (Transformation|GetWorldLocation _sphere) (Variables|/Script/Engine.SphereComponent|GetSphereRadius _sphere) (Utilities|Array|MakeArray "ObjectTypeQuery2") 0))
  (bind _array_element (Utilities|Array|ForEachLoopwithBreak _outactors :!label _label)
    (:LoopBody
      (if (Utilities|DoesObjectImplementInterface _array_element "/Game/Interface/BurnInterface.BurnInterface_C")
        (Class|BurnInterface|Burn(Message) _array_element)
        (if (Class|KismetMathLibrary|LinearColorIsNearEqual _returnvalue "(R=0.533333,G=0.011765,B=0.000000,A=1.000000)" 0.1)
          (Rendering|Components|Light|SetLightColor (Variables|Default|GetPointLight) "(R=1.000000,G=0.768628,B=0.000000,A=1.000000)" true)
          (Variables|Default|SetUnlocked false)
          (goto _label Break)
          (elif (Class|KismetMathLibrary|LinearColorIsNearEqual _returnvalue "(R=1.000000,G=0.768628,B=0.000000,A=1.000000)" 0.1)
            (Rendering|Components|Light|SetLightColor (Variables|Default|GetPointLight) "(R=0.031373,G=0.415686,B=0.000000,A=1.000000)" true)
            (Variables|Default|SetUnlocked false)
            (goto _label Break)
            (elif (Class|KismetMathLibrary|LinearColorIsNearEqual _returnvalue "(R=0.031373,G=0.415686,B=0.000000,A=1.000000)" 0.1)
              (Rendering|Components|Light|SetLightColor (Variables|Default|GetPointLight) "(R=0.533333,G=0.011765,B=0.000000,A=1.000000)" true)
              (Variables|Default|SetUnlocked true)
              (goto _label Break))))))))

(fn ConstructionScript)