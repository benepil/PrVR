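; BP_RibCage is a rib cage bone prop in Level 6 that a motion controller can grab, release and burn.
; Grab attaches it to the controller with world transforms kept and turns off physics on BoneMesh.
; Release clears the controller reference, detaches the prop and turns physics back on.
; Burn detaches it from any holding controller, then destroys the actor.
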(event EventBeginPlay)

(event Collision|EventActorBeginOverlap
  (params (OtherActor :type Actor%20Object%20Reference)))

(event EventTick
  (params (DeltaSeconds :type Float%20%28single-precision%29)))

(event EventRelease
  (params (Component :type Motion%20Controller%20Component%20Object%20Reference))
  (Variables|Default|SetMotionController 0)
  (Transformation|DetachFromActor "KeepWorld" "KeepWorld" "KeepWorld")
  (Physics|SetSimulatePhysics (Variables|Default|GetBoneMesh) true))

(event EventGrab
  (params (Component :type Motion%20Controller%20Component%20Object%20Reference))
  (bind _output_get (Variables|Default|SetMotionController Component))
  (Transformation|AttachComponentToComponent _output_get "None" "KeepWorld" "KeepWorld" "KeepWorld" true)
  (Physics|SetSimulatePhysics (Variables|Default|GetBoneMesh) false))

(event EventBurn
  (Utilities|IsValid (Variables|Default|GetMotionController)
    (:Is%20Valid
      (Variables|Default|SetMotionController 0)
      (Transformation|DetachFromActor "KeepWorld" "KeepWorld" "KeepWorld"))
    (:Is%20Not%20Valid
      _))
  (Actor|DestroyActor))

(fn ConstructionScript)