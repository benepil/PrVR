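; Grabbable lever for Level 2 that sets a Locked flag from its handle position.
; Grab stores the hand component when it is within the sphere's radius, and Release clears it.
; While held, Tick sets a clamped look-at roll, but an always-true branch immediately snaps the handle to 135 degrees and unlocks.
; When not held, a handle roll within 80 degrees of zero snaps to 45 and locks.
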(event EventBeginPlay)

(event Collision|EventActorBeginOverlap
  (params (OtherActor :type Actor%20Object%20Reference)))

(event EventGrab
  (params (Component :type Motion%20Controller%20Component%20Object%20Reference))
  (bind _sphere (Variables|Default|GetSphere))
  (if (Utilities|Operators|EqualEqual (Transformation|GetWorldLocation Component) (Transformation|GetWorldLocation _sphere) (Variables|/Script/Engine.SphereComponent|GetSphereRadius _sphere))
    (Variables|Default|SetHand Component)))

(event EventRelease
  (params (Component :type Motion%20Controller%20Component%20Object%20Reference))
  (if (== Component (Variables|Default|GetHand))
    (Variables|Default|SetHand 0)))

(event EventTick
  (params (DeltaSeconds :type Float%20%28single-precision%29))
  (bind _handle_bar (Variables|Default|GetHandle_Bar))
  (bind _hand (Variables|Default|GetHand))
  (Utilities|IsValid _hand
    (:Is%20Valid
      (Transformation|SetWorldRotation _handle_bar (Math|Rotator|MakeRotator (Math|Float|ClampAngle (- (.roll (Math|Rotator|FindLookatRotation (Transformation|GetWorldLocation _hand) (Transformation|GetWorldLocation _handle_bar))) 9e+01) 45.0 135.0) 0.0 2.7e+02) false false)
      (if true
        (Transformation|SetWorldRotation (Variables|Default|GetHandle_Bar) "0.000000,270.000000,135.000000" false false)
        (Variables|Default|SetLocked false)))
    (:Is%20Not%20Valid
      (if (Math|Float|NearlyEqual(Float) (.roll (Transformation|GetWorldRotation _handle_bar)) 0.0 8e+01)
        (Transformation|SetWorldRotation _handle_bar "0.000000,270.000000,45.000000" false false)
        (Variables|Default|SetLocked true)))))

(fn ConstructionScript)