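; Left-hand door in Level 2 that swings on its yaw axis to follow a component that grabs it.
; Grab stores the component as Hand if it is within the capsule's radius, and Release clears it.
; While held, Tick turns DoorWin with a look-at yaw clamped to a half-turn range; when free, it snaps shut if nearly closed.
; The Locked logic is unconnected and never runs.
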(event EventGrab
  (params (Component :type Motion%20Controller%20Component%20Object%20Reference))
  (bind _capsule (Variables|Default|GetCapsule))
  (if (Utilities|Operators|EqualEqual (Transformation|GetWorldLocation Component) (Transformation|GetWorldLocation _capsule) (Variables|/Script/Engine.CapsuleComponent|GetCapsuleRadius _capsule))
    (Variables|Default|SetHand Component)))

(event EventRelease
  (params (Component :type Motion%20Controller%20Component%20Object%20Reference))
  (if (== Component (Variables|Default|GetHand))
    (Variables|Default|SetHand 0)))

(event EventTick
  (params (DeltaSeconds :type Float%20%28single-precision%29))
  (bind _door_win (Variables|Default|GetDoor_Win))
  (bind _hand (Variables|Default|GetHand))
  (Utilities|IsValid _hand
    (:Is%20Valid
      (Transformation|SetWorldRotation _door_win (Math|Rotator|MakeRotator 0.0 0.0 (Math|Float|ClampAngle (- (.yaw (Math|Rotator|FindLookatRotation (Transformation|GetWorldLocation _hand) (Transformation|GetWorldLocation _door_win))) -9e+01) -9e+01 9e+01)) false false))
    (:Is%20Not%20Valid
      (if (Math|Float|NearlyEqual(Float) (.yaw (Transformation|GetWorldRotation _door_win)) 0.0 1e+01)
        (Transformation|SetWorldRotation _door_win "0, 0, 0" false false)))))

(fn ConstructionScript)