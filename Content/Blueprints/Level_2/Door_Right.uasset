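; Grabbable hinged door for Level 2, the right-hand one by name, that swings to follow the component grabbing it.
; Grab stores the component as Hand if it is within the Sphere's radius, and Release from that same component clears it.
; Tick yaws the Door from a look-at toward Hand, clamped to 90 degrees either way, or snaps it shut when released nearly closed.
; The Locked logic is disconnected and never runs.
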(event EventBeginPlay)

(event Collision|EventActorBeginOverlap
  (params (OtherActor :type Actor%20Object%20Reference)))

(event EventGrab
  (params (Component :type Motion%20Controller%20Component%20Object%20Reference))
  (bind _sphere (Variables|Default|GetSphere))
  (if (Utilities|Operators|EqualEqual (Transformation|GetWorldLocation Component) (Transformation|GetWorldLocation _sphere) (Variables|/Script/Engine.SphereComponent|GetSphereRadius _sphere))
    (Variables|Default|SetHand Component)))

(event EventRelease
  (params (Component :type Motion%20Controller%20Component%20Object%20Reference))
  (if (== Component (Variables|Default|GetHand))
    (Variables|Default|SetHand 0)))

(event EventTick
  (params (DeltaSeconds :type Float%20%28single-precision%29))
  (bind _door (Variables|Default|GetDoor))
  (bind _hand (Variables|Default|GetHand))
  (Utilities|IsValid _hand
    (:Is%20Valid
      (Transformation|SetWorldRotation _door (Math|Rotator|MakeRotator 0.0 0.0 (Math|Float|ClampAngle (- (.yaw (Math|Rotator|FindLookatRotation (Transformation|GetWorldLocation _hand) (Transformation|GetWorldLocation _door))) 9e+01) -9e+01 9e+01)) false false))
    (:Is%20Not%20Valid
      (if (Math|Float|NearlyEqual(Float) (.yaw (Transformation|GetWorldRotation _door)) 0.0 1e+01)
        (Transformation|SetWorldRotation _door "0, 0, 0" false false)))))

(fn ConstructionScript)