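; Level 5 lever that a hand component can grab within its sphere and that tracks a Locked state.
; Grab and Release set or clear the Hand reference.
; While held, Tick derives a clamped pitch from the hand-to-pivot look-at, but an always-true branch immediately overrides it with a fixed rotation and clears Locked.
; When not held, a pitch near zero snaps the lever to rest and sets Locked.
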(event EventBeginPlay)

(event Collision|EventActorBeginOverlap
  (params (OtherActor :type Actor%20Object%20Reference)))

(event EventGrab
  (params (Component :type Motion%20Controller%20Component%20Object%20Reference))
  (bind _sphere (Variables|Default|GetSphere))
  (if (Utilities|Operators|EqualEqual (Transformation|GetWorldLocation Component) (Transformation|GetWorldLocation _sphere) (Variables|/Script/Engine.SphereComponent|GetSphereRadius _sphere))
    (Variables|Default|SetHand Component)))

(event EventRelease
  (params (Component :type Motion%20Controller%20Component%20Object%20Reference))
  (if (== Component (Variables|Default|GetHand))
    (Variables|Default|SetHand 0)))

(event EventTick
  (params (DeltaSeconds :type Float%20%28single-precision%29))
  (bind _scene (Variables|Default|GetScene))
  (bind _hand (Variables|Default|GetHand))
  (Utilities|IsValid _hand
    (:Is%20Valid
      (Transformation|SetWorldRotation _scene (Math|Rotator|MakeRotator 0.0 (Math|Float|ClampAngle (- (.pitch (Math|Rotator|FindLookatRotation (Transformation|GetWorldLocation _hand) (Transformation|GetWorldLocation _scene))) 45.0) 0.0 9e+01) 2.7e+02) false false)
      (if true
        (Transformation|SetWorldRotation (Variables|Default|GetScene) "270.000000,0.000000,0.000000" false false)
        (Variables|Default|SetLocked false)))
    (:Is%20Not%20Valid
      (if (Math|Float|NearlyEqual(Float) (.pitch (Transformation|GetWorldRotation _scene)) 0.0 1e+01)
        (Transformation|SetWorldRotation _scene "0.000000,270.000000,0.000000" false false)
        (Variables|Default|SetLocked true)))))

(fn ConstructionScript)